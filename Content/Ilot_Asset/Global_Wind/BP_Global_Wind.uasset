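; Global wind actor that pushes wind speed, intensity and the Arrow component's forward direction into the MPC_Global_Wind material parameter collection.
; GlobalWind writes these values from the construction script, so edits preview in the editor, and again from a looping timer started on BeginPlay.
; When StopWind is set, the timer callback clears the timer and resets speed and intensity to fixed values while keeping the arrow's direction.
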(event `self.ReceiveBeginPlay`
  (`self.StartTimer`))

(event `StartTimer`
  (bind _returnvalue (`KismetSystemLibrary.K2_SetTimerDelegate` (delegate `Le code`) 1.5 true)))

(event `Le code`
  (`self.Global_Wind`)
  (if (`self.StopWind`)
    (`KismetSystemLibrary.K2_ClearAndInvalidateTimerHandle` (stale `StartTimer` _returnvalue))
    (`KismetMaterialLibrary.SetScalarParameterValue` "/Game/Ilot_Asset/Global_Wind/MPC_Global_Wind.MPC_Global_Wind" "Wind_Speed" 0.5)
    (`KismetMaterialLibrary.SetScalarParameterValue` "/Game/Ilot_Asset/Global_Wind/MPC_Global_Wind.MPC_Global_Wind" "Wind_Intensity" 0.5)
    (`KismetMaterialLibrary.SetVectorParameterValue` "/Game/Ilot_Asset/Global_Wind/MPC_Global_Wind.MPC_Global_Wind" "Wind_Direction" (`KismetMathLibrary.Conv_VectorToLinearColor` (`SceneComponent.GetForwardVector` (`self.Arrow`))))))

(fn `Global_Wind`
  (`KismetMaterialLibrary.SetScalarParameterValue` "/Game/Ilot_Asset/Global_Wind/MPC_Global_Wind.MPC_Global_Wind" "Wind_Speed" (`self.Wind_Speed`))
  (`KismetMaterialLibrary.SetScalarParameterValue` "/Game/Ilot_Asset/Global_Wind/MPC_Global_Wind.MPC_Global_Wind" "Wind_Intensity" (`self.Wind_Intensity`))
  (`KismetMaterialLibrary.SetVectorParameterValue` "/Game/Ilot_Asset/Global_Wind/MPC_Global_Wind.MPC_Global_Wind" "Wind_Direction" (`KismetMathLibrary.Conv_VectorToLinearColor` (`SceneComponent.GetForwardVector` (`self.Arrow`)))))

(fn `UserConstructionScript`
  (`self.Global_Wind`))